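; Shield projectile that grows on a looping timer and launches non-player characters with force multiplied by its scale.
; Its first non-character hit fires an impact event, scaled effect and sound, then stops growth.
; ReturnToPlayer switches collision to overlap and lerps it toward the player via timeline, still launching characters it overlaps.
; Overlapping the player, or a delay started during that timeline, notifies of the return and destroys it.
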(event OnComponentBeginOverlap(BoxCollision)
  (params (OverlappedComponent :type Primitive%20Component%20Object%20Reference) (OtherActor :type Actor%20Object%20Reference) (OtherComp :type Primitive%20Component%20Object%20Reference) (OtherBodyIndex :type Integer) (bFromSweep :type Boolean) (SweepResult :type Hit%20Result%20Structure%20%28by%20ref%29))
  ;[1 1 1] Overlap
  (Utilities|Casting|CastToBP_Player OtherActor
    (:then
      (if (Variables|Default|GetReturningToPlayer)
        (CallFunction|CallReturned)))
    (:CastFailed
      (bind _ascharacter (Utilities|Casting|CastToCharacter OtherActor))
      (Character|LaunchCharacter _ascharacter (* (Variables|Default|GetCharacterLaunch) (Variables|Default|GetScale)) true true))))

(event OnComponentHit(BoxCollision)
  (params (HitComponent :type Primitive%20Component%20Object%20Reference) (OtherActor :type Actor%20Object%20Reference) (OtherComp :type Primitive%20Component%20Object%20Reference) (NormalImpulse :type Vector :default "0, 0, 0") (Hit :type Hit%20Result%20Structure%20%28by%20ref%29))
  (bind _impactpoint (Collision|BreakHitResult Hit))
  ;[1 1 1] On Impact
  (bind _ascharacter (Utilities|Casting|CastToCharacter OtherActor)
    (:then
      (Utilities|Casting|CastToBP_Player _ascharacter
        (:CastFailed
          (Development|PrintString "NPC")
          (Character|LaunchCharacter _ascharacter (* (Variables|Default|GetCharacterLaunch) (Variables|Default|GetScale)) true true))))
    (:CastFailed
      (Development|PrintString "NOT A CHARACTER")
      (Utilities|FlowControl|DoOnce false
        (:Completed
          (Default|CallOnProjectileImpact 0 Hit)
          (CallFunction|SpawnImpactEffect _impactpoint)
          (CallFunction|PlayImpactSound _impactpoint)
          (CallFunction|StopGrowth))))))

(event Custom|Grow
  ;[1 1 1] Growth
  (if (Variables|Default|GetIsGrowing)
    (bind _output_get (Variables|Default|SetScale (+ (Transformation|GetActorScale3D) (Variables|Default|GetGrowthRate))))
    (Transformation|SetActorScale3D _output_get)))

(event Custom|StopGrowth
  ;[1 1 1] Growth
  (if (Variables|Default|GetIsGrowing)
    (Utilities|Time|ClearandInvalidateTimerbyHandle (Variables|Default|GetGrowthTimer))
    (Variables|Default|SetIsGrowing false)))

(event Custom|ReturnToPlayer
  ;[1 1 1] Return To Player
  (Variables|Default|SetReturningToPlayer true)
  (Collision|SetCollisionResponsetoAllChannels (Variables|Default|GetBoxCollision) "ECR_Overlap")
  (CallFunction|StopGrowth)
  (bind _newtrack_0 (Timeline|MoveShield Play)
    (:Update
      (Transformation|SetActorLocation (Math|Vector|Lerp(Vector) (Transformation|GetActorLocation) (Transformation|GetActorLocation (Game|GetPlayerCharacter 0)) _newtrack_0) true false)
      (Utilities|FlowControl|Delay 1.0)
      (CallFunction|CallReturned))))

(event Custom|CallReturned
  (Default|CallReturnedtoPlayer)
  (Actor|DestroyActor))

(event EventBeginPlay
  ;[1 1 1] On Spawn
  (|CallParentFunction)
  (bind _returnvalue (Utilities|Time|SetTimerbyEvent (EventDispatchers|CreateEvent :!event Custom|Grow) (Variables|Default|GetGrowthInterval) true))
  (Variables|Default|SetGrowthTimer _returnvalue))

(event EventSpawnImpactEffect
  (params (Location :type Vector :default "0, 0, 0"))
  ;[1 1 1] Impact Effect
  (bind _impacteffect (Variables|Default|GetImpactEffect)
    (:then
      (Effects|SpawnEmitteratLocation _impacteffect Location "0, 0, 0" (Variables|Default|GetScale)))
    (:else)))

(fn ConstructionScript
  (|CallParentFunction))