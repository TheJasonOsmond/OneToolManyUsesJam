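; BP_PressureDoor is a door that rises and lowers in response to pressure plates.
; On BeginPlay it binds its raise and lower events to every BP_PressurePlate in the level, with no per-door pairing.
; Both events set IsOpen, play a sound at the door, then play or reverse a shared Timeline.
; The Timeline lerps the Door component's relative Z height with sweep enabled.
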(event Custom|RaiseDoor
  (Variables|Default|SetIsOpen true)
  (Audio|PlaySoundatLocation "/Engine/EditorSounds/GamePreview/EndPlayInEditor.EndPlayInEditor" (Transformation|GetActorLocation) "0, 0, 0" 1.0 1.0 0.0 0 0 0 0)
  (if (Variables|Default|GetIsOpen)
    (bind _height (Timeline|Timeline Play)
      (:Update
        (Transformation|SetRelativeLocation (Variables|Default|GetDoor) (Math|Vector|MakeVector 0.0 0.0 (Math|Float|Lerp 0.0 7e+02 _height)) true false)))
    (else
      (Timeline|Timeline Reverse))))

(event Custom|LowerDoor
  (Variables|Default|SetIsOpen false)
  (Audio|PlaySoundatLocation "/Engine/EditorSounds/GamePreview/EndPlayInEditor.EndPlayInEditor" (Transformation|GetActorLocation) "0, 0, 0" 1.0 1.0 0.0 0 0 0 0)
  (if (Variables|Default|GetIsOpen)
    (bind _height (Timeline|Timeline Play)
      (:Update
        (Transformation|SetRelativeLocation (Variables|Default|GetDoor) (Math|Vector|MakeVector 0.0 0.0 (Math|Float|Lerp 0.0 7e+02 _height)) true false)))
    (else
      (Timeline|Timeline Reverse))))

(event EventBeginPlay
  (bind _outactors (Actor|GetAllActorsOfClass "/Game/ShieldGame/Objects/BP_PressurePlate.BP_PressurePlate_C"))
  (for _array_element _outactors
    ;[1 1 1] Raise
    (EventDispatchers|BindEventtoRaiseDoor _array_element (EventDispatchers|CreateEvent :!event Custom|RaiseDoor))
    ;[1 1 1] Lower
    (EventDispatchers|BindEventtoLowerDoor _array_element (EventDispatchers|CreateEvent :!event Custom|LowerDoor))))

(fn ConstructionScript)